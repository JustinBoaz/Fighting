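; Cosmetic effects component for a fighter that handles landing sounds, camera shakes and stopping montages on crouch.
; On Tick, each new grounding fires a weak or heavy impact with sound and medium or strong shake, chosen by WeakGrounded.
; Shake events set a type briefly via retriggerable delay; Tick replays it at a per-type scale when player zero is the fighter or its target.
; Crouching stops the current montage after a short delay.
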(event `self.ReceiveBeginPlay`
  (`parent.ReceiveBeginPlay`))

(event `Break Ground Weak`
  (bind _fighter (`self.Fighter`))
  (`/Game/UltimateFightingGameEngine/Blueprints/UFGE_BaseCharacter.Play Sound` _fighter null (`Actor.K2_GetActorLocation` _fighter) 1.0)
  (`self.Play Medium CS`))

(event `self.cBegin Play`)

(event `Break Ground`
  (bind _fighter (`self.Fighter`))
  (`/Game/UltimateFightingGameEngine/Blueprints/UFGE_BaseCharacter.Play Sound` _fighter (`/Game/UltimateFightingGameEngine/Blueprints/SoundEffects.Hit Ground SFX`) (`Actor.K2_GetActorLocation` _fighter) 1.5)
  (`self.Play Strong CS`))

(event `Play Weak CS`
  (set `self.Camera Shake` "NewEnumerator1")
  (`KismetSystemLibrary.RetriggerableDelay` 0.21)
  (set `self.Camera Shake` "NewEnumerator0"))

(event `Play Medium CS`
  (set `self.Camera Shake` "NewEnumerator2")
  (`KismetSystemLibrary.RetriggerableDelay` 0.21)
  (set `self.Camera Shake` "NewEnumerator0"))

(event `Play Strong CS`
  (set `self.Camera Shake` "NewEnumerator3")
  (`KismetSystemLibrary.RetriggerableDelay` 0.21)
  (set `self.Camera Shake` "NewEnumerator0"))

(event `Play Gun CS`
  (set `self.Camera Shake` "NewEnumerator4")
  (`KismetSystemLibrary.RetriggerableDelay` 0.21)
  (set `self.Camera Shake` "NewEnumerator0"))

(event `self.ReceiveTick`
  (params (DeltaSeconds :type "Float (single-precision)"))
  (bind _returnvalue (`GameplayStatics.GetPlayerCameraManager` 0))
  (`self.Crouch Montage Event`)
  (`|ExecutionSequence`
    (:`then_0`
      (bind _returnvalue_2 (`self.Dealing With Player`))
      (if _returnvalue_2
        (switch `/Game/UltimateFightingGameEngine/Blueprints/Enums/CameraShake` (`self.Camera Shake`)
          (:`NewEnumerator1`
            (`PlayerCameraManager.PlayCameraShake` :`self` _returnvalue :`ShakeClass` "/Game/UltimateFightingGameEngine/Blueprints/Misc/CameraShake.CameraShake_C" :`Scale` 0.3))
          (:`NewEnumerator2`
            (`PlayerCameraManager.PlayCameraShake` :`self` _returnvalue :`ShakeClass` "/Game/UltimateFightingGameEngine/Blueprints/Misc/CameraShake.CameraShake_C" :`Scale` 0.6))
          (:`NewEnumerator3`
            (`PlayerCameraManager.PlayCameraShake` :`self` _returnvalue :`ShakeClass` "/Game/UltimateFightingGameEngine/Blueprints/Misc/CameraShake.CameraShake_C"))
          (:`NewEnumerator4`
            (`PlayerCameraManager.PlayCameraShake` :`self` _returnvalue :`ShakeClass` "/Game/UltimateFightingGameEngine/Blueprints/Misc/CameraShake.CameraShake_C" :`Scale` 1.5)))))
    (:`then_1`
      (if (`/Game/UltimateFightingGameEngine/Blueprints/FightingBaseComponent.Grounded?` (`self.FBC`))
        (`/Engine/EditorBlueprintResources/StandardMacros.DoOnce` false :!label _label
          (:`Completed`
            (if (`self.Weak Grounded?`)
              (`self.Break Ground Weak`)
              (set `self.Weak Grounded?` false)
              (else
                (`self.Break Ground`)))))
        (else
          (goto _label :!via `Reset`))))))

(event `Crouch Montage Event`
  (if (`/Game/UltimateFightingGameEngine/Blueprints/UFGE_BaseCharacter.Crouching?` (`self.Fighter`))
    (`/Engine/EditorBlueprintResources/StandardMacros.DoOnce` false :!label _label_2
      (:`Completed`
        (`KismetSystemLibrary.RetriggerableDelay` 0.1)
        (`/Game/UltimateFightingGameEngine/Blueprints/UFGE_BaseCharacter.Stop Montage` (`self.Fighter`) null)))
    (else
      (goto _label_2 :!via `Reset`))))

(fn `Dealing With Player`
  (returns (ReturnValue :type Boolean))
  (bind _returnvalue (`GameplayStatics.GetPlayerCharacter` 0))
  (bind _fbc (`self.FBC`))
  (return (or (== (`/Game/UltimateFightingGameEngine/Blueprints/BaseComponent.Fighter` _fbc) _returnvalue) (== (`/Game/UltimateFightingGameEngine/Blueprints/FightingBaseComponent.Target` _fbc) _returnvalue))))