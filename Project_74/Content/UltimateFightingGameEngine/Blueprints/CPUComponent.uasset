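; CPU opponent component that drives non-player fighters by faking input on the fighting base component; it destroys itself on player fighters.
; Tick runs fight logic while a target exists, resetting during hit montages, and otherwise heads for the nearest AI checkpoint.
; Distance selects movement, by axis or double-tapped key, or delayed attacks using random single-button moves.
; Attacks yield when the target is already attacking, with retriggerable timers resetting combat state.
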(event `Add Random Key`
  (params (Delay :type "Float (double-precision)"))
  (bind _fighter (`self.Fighter`))
  (`KismetSystemLibrary.Delay` Delay)
  (switch `int` (`KismetMathLibrary.RandomIntegerInRange` 0 1)
    (:`0`
      (`/Game/UltimateFightingGameEngine/Blueprints/UFGE_BaseCharacter.Add Key` _fighter "NewEnumerator5" true))
    (:`1`
      (`/Game/UltimateFightingGameEngine/Blueprints/UFGE_BaseCharacter.Add Key` _fighter "NewEnumerator6" true))))

(event `self.cBegin Play`
  ;[1 0.4631 0] Begin Play
  (`KismetSystemLibrary.Delay` 0.2)
  (if (`/Game/UltimateFightingGameEngine/Blueprints/UFGE_BaseCharacter.Is Player?` (`self.Fighter`))
    (`self.K2_DestroyComponent`)))

(event `self.ReceiveTick`
  (params (DeltaSeconds :type "Float (single-precision)"))
  (bind _fighter (`self.Fighter`))
  (bind _fighter_2 (`self.Fighter`))
  (bind _fighter_3 (`self.Fighter`))
  (bind _target (`/Game/UltimateFightingGameEngine/Blueprints/FightingBaseComponent.Target` (`self.FBC`)))
  (bind _target_2 (`/Game/UltimateFightingGameEngine/Blueprints/FightingBaseComponent.Target` (`/Game/UltimateFightingGameEngine/Blueprints/UFGE_BaseCharacter.FightingBaseComponent` (`self.Fighter`))))
  (if (> (`Actor.GetGameTimeSinceCreation` (`self.Fighter`)) 0.4)
    (`|ExecutionSequence`
      (:`then_0`
        (if (not (`/Game/UltimateFightingGameEngine/Blueprints/UFGE_BaseCharacter.Dead?` _fighter_2))
          (`/Game/UltimateFightingGameEngine/Blueprints/FightingBaseComponent.Target` (`/Game/UltimateFightingGameEngine/Blueprints/UFGE_BaseCharacter.FightingBaseComponent` _fighter_2)
            (:`then`
              (set `/Game/UltimateFightingGameEngine/Blueprints/UFGE_BaseCharacter.Fighting?` true _fighter_2)
              (bind _returnvalue (`Character.GetCurrentMontage` _fighter_2))
              (bind _values (`BlueprintMapLibrary.Map_Values` (break `/Game/UltimateFightingGameEngine/Blueprints/Structs/HitMontagesMap` (`BlueprintMapLibrary.Map_Find` (`/Game/UltimateFightingGameEngine/Blueprints/UFGE.Hit Montages` (`/Game/UltimateFightingGameEngine/Blueprints/FightingBaseComponent.UFGE` (`/Game/UltimateFightingGameEngine/Blueprints/UFGE_BaseCharacter.FightingBaseComponent` _fighter_3))) (`/Game/UltimateFightingGameEngine/Blueprints/UFGE_BaseCharacter.Character` _fighter_3)))))
              (if (`KismetArrayLibrary.Array_Contains` _values _returnvalue)
                (`KismetArrayLibrary.Array_Clear` (`/Game/UltimateFightingGameEngine/Blueprints/FightingBaseComponent.Keys Pressed` (`/Game/UltimateFightingGameEngine/Blueprints/UFGE_BaseCharacter.FightingBaseComponent` (`self.Fighter`))))
                (`self.Reset Combat`)
                (`self.Reset Just Attacked`)
                (elif (not (and (`/Game/UltimateFightingGameEngine/Blueprints/FightingBaseComponent.Move Camera` (`/Game/UltimateFightingGameEngine/Blueprints/UFGE_BaseCharacter.FightingBaseComponent` _target_2)) (`/Game/UltimateFightingGameEngine/Blueprints/UFGE_BaseCharacter.Is Player?` _target_2)))
                  (`|ExecutionSequence`
                    (:`then_0`
                      (if (< (`Actor.GetDistanceTo` _fighter _target) (+ (* (`KismetMathLibrary.Conv_BoolToDouble` (`/Game/UltimateFightingGameEngine/Blueprints/UFGE_BaseCharacter.Is Player?` _target)) 60.0) 115.0))
                        (`self.Base Combat`)
                        (else
                          (`self.Movement`)
                          (`self.Reset Combat`))))
                    (:`then_1`
                      (`KismetSystemLibrary.Delay` 3.0)
                      (set `self.Movement Type A?` (`KismetMathLibrary.Conv_IntToBool` (`KismetMathLibrary.RandomIntegerInRange` 0 1)))))
                  (else
                    (set `/Game/UltimateFightingGameEngine/Blueprints/UFGE_BaseCharacter.RightAxisValue` 0.0 _fighter)))))
            (:`else`
              (`self.End Fight`))))))))

(event `Movement`
  (bind _fbc (`self.FBC`))
  (if (or (`self.Movement Type A?`) (< (`Actor.GetDistanceTo` (`self.Fighter`) (`/Game/UltimateFightingGameEngine/Blueprints/FightingBaseComponent.Target` (`self.FBC`))) 120.0))
    (set `/Game/UltimateFightingGameEngine/Blueprints/UFGE_BaseCharacter.RightAxisValue` 1.0 (`self.Fighter`))
    (else
      (set `/Game/UltimateFightingGameEngine/Blueprints/FightingBaseComponent.Keys Pressed` (`|MakeArray` "NewEnumerator3" "NewEnumerator3" :!type "/Game/UltimateFightingGameEngine/Blueprints/Enums/Keys Enum") _fbc)
      (`KismetSystemLibrary.Delay` 0.1)
      (set `self.Movement Type A?` true)
      (`KismetArrayLibrary.Array_Clear` (`/Game/UltimateFightingGameEngine/Blueprints/FightingBaseComponent.Keys Pressed` _fbc)))))

(event `Base Combat`
  (bind _fbc (`self.FBC`))
  (bind _target (`/Game/UltimateFightingGameEngine/Blueprints/FightingBaseComponent.Target` _fbc))
  (`|ExecutionSequence`
    (:`then_0`
      (set `/Game/UltimateFightingGameEngine/Blueprints/UFGE_BaseCharacter.RightAxisValue` 0.0 (`self.Fighter`))
      (`/Engine/EditorBlueprintResources/StandardMacros.DoOnce` false :!label _label
        (:`Completed`
          (`KismetSystemLibrary.RetriggerableDelay` 1.0)
          (`/Game/UltimateFightingGameEngine/Blueprints/FightingBaseComponent.Reset Keys` _fbc)
          (`/Engine/EditorBlueprintResources/StandardMacros.IsValid` _target
            (:`Is Valid`
              (bind _returnvalue (`self.Combat State Checker` :!label _label_2))
              (if _returnvalue
                (if (not (and (> (`Actor.GetDistanceTo` (`self.Fighter`) _target) 110.0) (`/Game/UltimateFightingGameEngine/Blueprints/UFGE_BaseCharacter.Is Player?` _target)))
                  (`self.Key Attack`))))))))
    (:`then_1`
      (`KismetSystemLibrary.RetriggerableDelay` 1.0)
      (`self.Reset Combat`))))

(event `Key Attack`
  (bind _target (`/Game/UltimateFightingGameEngine/Blueprints/FightingBaseComponent.Target` (`self.FBC`)))
  (`self.Combat State SR`)
  (`/Engine/EditorBlueprintResources/StandardMacros.IsValid` _target
    (:`Is Valid`
      (bind _returnvalue (`Character.GetCurrentMontage` _target))
      (bind _montages (`/Game/UltimateFightingGameEngine/Blueprints/FightingBaseComponent.Get All Attack Montages` (`/Game/UltimateFightingGameEngine/Blueprints/UFGE_BaseCharacter.FightingBaseComponent` _target)))
      (if (`KismetArrayLibrary.Array_Contains` _montages _returnvalue)
        (`self.Stop Attack Montage`)
        (elif (not (`self.Just Attacked?`))
          (bind _result (`self.Simple AI Attack`))
          (set `/Game/UltimateFightingGameEngine/Blueprints/FightingBaseComponent.Keys Pressed` _result (`self.FBC`))
          (set `self.Just Attacked?` true)
          (`self.Reset Just Attacked`)
          (`KismetSystemLibrary.Delay` (* (`KismetArrayLibrary.Array_Length` _result) 0.2))
          (`KismetArrayLibrary.Array_Clear` (`/Game/UltimateFightingGameEngine/Blueprints/FightingBaseComponent.Keys Pressed` (`self.FBC`)))
          (`self.Reset Combat`))))))

(event `Reset Just Attacked`
  (if (`/Game/UltimateFightingGameEngine/Blueprints/FightingBaseComponent.Can Cancel?` (`self.FBC`))
    (set `self.Just Attacked?` false)
    (`self.Reset Combat`)
    (else
      (`KismetSystemLibrary.Delay` 0.1)
      (`self.Reset Just Attacked`))))

(event `Reset Combat`
  (goto _label :!via `Reset`))

(event `Restore Combat State`
  (`KismetSystemLibrary.Delay` 0.1)
  (goto _label_2))

(event `Combat State SR`
  (`KismetSystemLibrary.RetriggerableDelay` 1.5)
  (`self.Reset Combat`)
  (`self.Reset Just Attacked`))

(event `End Fight`
  ;[0 1 0] End Fight Event
  (`self.Move To Checkpoint`)
  (`KismetSystemLibrary.Delay` 0.2)
  (set `/Game/UltimateFightingGameEngine/Blueprints/UFGE_BaseCharacter.Fighting?` false (`self.Fighter`))
  (`/Game/UltimateFightingGameEngine/Blueprints/FightingBaseComponent.Reset Keys` (`self.FBC`)))

(event `Move To Checkpoint`
  ;[0 1 0] End Fight Event
  ;;[1 1 1] Move AI To Checkpoint
  (if (not (`/Game/UltimateFightingGameEngine/Blueprints/UFGE_BaseCharacter.Fighting?` (`self.Fighter`)))
    (bind _outactors (`GameplayStatics.GetAllActorsOfClass` "/Game/UltimateFightingGameEngine/Blueprints/Other/AICheckpoint.AICheckpoint_C"))
    (for _array_element _outactors
      (bind _returnvalue (`Actor.GetDistanceTo` _array_element (`self.Fighter`)))
      (if (< _returnvalue (`self.Distance To Beat`))
        (set `self.Distance To Beat` _returnvalue)
        (set `self.Checkpoint` _array_element)))
    (bind _checkpoint (`self.Checkpoint`)
      (:`then`
        (`self.Move To ( CPU )` _checkpoint)
        (if (> (`self.Distance To Beat`) (`self.Default Distance`))
          (set `self.Distance To Beat` (`self.Default Distance`) :!label _label_3)))
      (:`else`
        (goto _label_3)))))

(fn `Animation Changer`
  (params (`Combo To Check` :type "/Game/UltimateFightingGameEngine/Blueprints/Enums/Combos Enum" :default "NewEnumerator11"))
  (returns (Return :type "/Game/UltimateFightingGameEngine/Blueprints/Enums/Combos Enum"))
  (bind _target (`/Game/UltimateFightingGameEngine/Blueprints/FightingBaseComponent.Target` (`self.FBC`))
    (:`then`
      (if (`/Game/UltimateFightingGameEngine/Blueprints/UFGE_BaseCharacter.Is Player?` _target)
        (return `Combo To Check`)
        (else
          (return (`BlueprintMapLibrary.Map_Find` (`self.Combo Alternate`) `Combo To Check`)))))
    (:`else`
      (return "NewEnumerator13"))))

(fn `Combat State Checker`
  (returns (ReturnValue :type Boolean))
  (bind _fbc (`self.FBC`))
  (bind _returnvalue (`Character.GetCurrentMontage` (`self.Fighter`)))
  (bind _montages (`/Game/UltimateFightingGameEngine/Blueprints/FightingBaseComponent.Get All Attack Montages` _fbc))
  (return (`KismetMathLibrary.BooleanNOR` (`KismetArrayLibrary.Array_Contains` _montages _returnvalue) (`/Game/UltimateFightingGameEngine/Blueprints/FightingBaseComponent.In Hit Animation?` _fbc))))

(fn `Move To ( CPU )`
  (params (Goal :type "Actor Object Reference"))
  (bind _fighter (`self.Fighter`))
  (if (not (`/Game/UltimateFightingGameEngine/Blueprints/UFGE_BaseCharacter.Is Player?` _fighter))
    (`AIBlueprintHelperLibrary.SimpleMoveToActor` (`Pawn.GetController` _fighter) Goal)
    (return)))

(fn `Simple AI Attack`
  (returns (Result :type "Array of /Game/UltimateFightingGameEngine/Blueprints/Enums/Keys Enum"))
  (locals (Moveset :type "Array of /Game/UltimateFightingGameEngine/Blueprints/Structs/Moveset Structure"))
  (if (not (`self.Training Dummy?`))
    (set `local.Moveset` (`/Game/UltimateFightingGameEngine/Blueprints/FightingBaseComponent.Get Moveset` (`/Game/UltimateFightingGameEngine/Blueprints/UFGE_BaseCharacter.FightingBaseComponent` (`self.Fighter`))))
    (`KismetArrayLibrary.Array_Shuffle` (`local.Moveset`))
    (for _array_element (`local.Moveset`)
      (bind ((`ButtonCombination_26_AFEA2BC54F6EB20403E1F5BDD47FD24F` _buttoncombination)) (break `/Game/UltimateFightingGameEngine/Blueprints/Structs/Moveset` _array_element))
      (if (== (`KismetArrayLibrary.Array_Length` _buttoncombination) 1)
        (return _buttoncombination)))))

(fn `Stop Attack Montage`
  (bind _fighter (`self.Fighter`))
  (bind _returnvalue (`Character.GetCurrentMontage` _fighter))
  (bind _montages (`/Game/UltimateFightingGameEngine/Blueprints/FightingBaseComponent.Get All Attack Montages` (`self.FBC`)))
  (if (`KismetArrayLibrary.Array_Contains` _montages _returnvalue)
    (`Character.StopAnimMontage` _fighter null)
    (return)
    (else
      (return))))