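; AISpawner is a placed actor that spawns a CPU-controlled fighting game character at its own transform when play begins.
; It spawns a UFGE_BaseCharacter marked non-player, stores it as SpawnedActor, and passes on its Character setting.
; It then links itself to the character's CPUComponent as Spawner, creates the default controller, disables its own tick, and forwards its TrainingDummy setting.
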(event `self.ReceiveBeginPlay`
  (bind _returnvalue (`|SpawnActorFromClass` "/Game/UltimateFightingGameEngine/Blueprints/UFGE_BaseCharacter.UFGE_BaseCharacter_C" (`self.GetTransform`) "AdjustIfPossibleButAlwaysSpawn" "OverrideRootScale" null "Mannequin" null))
  (set `/Game/UltimateFightingGameEngine/Blueprints/UFGE_BaseCharacter.Is Player?` false _returnvalue)
  (set `self.Spawned Actor` _returnvalue)
  (set `/Game/UltimateFightingGameEngine/Blueprints/UFGE_BaseCharacter.Character` (`self.Character`) _returnvalue)
  (set `/Game/UltimateFightingGameEngine/Blueprints/CPUComponent.Spawner` self (`/Game/UltimateFightingGameEngine/Blueprints/UFGE_BaseCharacter.CPUComponent` _returnvalue))
  (`Pawn.SpawnDefaultController` _returnvalue)
  (`self.SetActorTickEnabled` false)
  (set `/Game/UltimateFightingGameEngine/Blueprints/CPUComponent.Training Dummy?` (`self.Training Dummy?`) (`/Game/UltimateFightingGameEngine/Blueprints/UFGE_BaseCharacter.CPUComponent` _returnvalue)))

(fn `UserConstructionScript`)