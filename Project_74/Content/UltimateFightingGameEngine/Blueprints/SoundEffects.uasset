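; SoundEffects declares a set of sound effect functions for a fighting game, apparently as a Blueprint interface.
; It has entry points for KO, strong, medium and weak hits, ground impacts, the countdown timer and the fight start.
; Every function takes no parameters and returns nothing, with no logic or audio playback in this file.
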(fn `Countdown Timer SFX`
  (returns (SFX :type "SoundWave Object Reference"))
  (return null))

(fn `Hit Ground SFX`
  (returns (SFX :type "SoundWave Object Reference"))
  (return null))

(fn `KO SFX`
  (returns (SFX :type "SoundWave Object Reference"))
  (return null))

(fn `Medium Hit SFX`
  (returns (SFX :type "SoundWave Object Reference"))
  (return null))

(fn `Start Fight SFX`
  (returns (SFX :type "SoundWave Object Reference"))
  (return null))

(fn `Strong Hit SFX`
  (returns (SFX :type "SoundWave Object Reference"))
  (return null))

(fn `Weak Hit SFX`
  (returns (SFX :type "SoundWave Object Reference"))
  (return null))