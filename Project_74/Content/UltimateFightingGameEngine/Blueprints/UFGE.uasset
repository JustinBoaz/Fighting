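; UFGE is an actor that holds and persists the fighting game engine's Characters, Movesets and HitMontages data.
; Save copies the three collections into a new SaveData object in the "UFGE" slot, and Load reads them back if that save casts successfully.
; ClearAllMovesets wipes all three, refills Movesets and Characters with numbered "Blank" placeholder keys, leaves HitMontages empty, then saves over the slot.
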(event `Clear All Movesets`
  ;[1 1 1] Reset All Moveset Values
  (`BlueprintMapLibrary.Map_Clear` (`self.Movesets`))
  (for _index (range 36)
    (`BlueprintMapLibrary.Map_Add` (`self.Movesets`) (`KismetStringLibrary.Concat_StrStr` (`KismetStringLibrary.Conv_IntToString` _index) " Blank")))
  (`BlueprintMapLibrary.Map_Clear` (`self.Characters`))
  (for _index_2 (range 501)
    (`BlueprintMapLibrary.Map_Add` (`self.Characters`) (`KismetStringLibrary.Concat_StrStr` (`KismetStringLibrary.Conv_IntToString` _index_2) " Blank")))
  (`BlueprintMapLibrary.Map_Clear` (`self.Hit Montages`))
  (`self.Save`))

(event `Load`
  (`GameplayStatics.CreateSaveGameObject` "/Game/UltimateFightingGameEngine/Blueprints/SaveData.SaveData_C")
  (bind _returnvalue (`GameplayStatics.LoadGameFromSlot` "UFGE"))
  (bind _assave_data (cast `/Game/UltimateFightingGameEngine/Blueprints/SaveData` _returnvalue))
  (set `self.Characters` (`/Game/UltimateFightingGameEngine/Blueprints/SaveData.Characters` _assave_data))
  (set `self.Movesets` (`/Game/UltimateFightingGameEngine/Blueprints/SaveData.Movesets` _assave_data))
  (set `self.Hit Montages` (`/Game/UltimateFightingGameEngine/Blueprints/SaveData.Hit Montages` _assave_data)))

(event `Save`
  (bind _returnvalue (`GameplayStatics.CreateSaveGameObject` "/Game/UltimateFightingGameEngine/Blueprints/SaveData.SaveData_C"))
  (set `/Game/UltimateFightingGameEngine/Blueprints/SaveData.Characters` (`self.Characters`) _returnvalue)
  (set `/Game/UltimateFightingGameEngine/Blueprints/SaveData.Movesets` (`self.Movesets`) _returnvalue)
  (set `/Game/UltimateFightingGameEngine/Blueprints/SaveData.Hit Montages` (`self.Hit Montages`) _returnvalue)
  (`GameplayStatics.SaveGameToSlot` _returnvalue "UFGE"))

(fn `UserConstructionScript`)